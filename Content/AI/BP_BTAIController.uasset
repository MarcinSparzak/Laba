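; BP_BTAIController is an AI controller that runs the BT_NPC behavior tree with the BB_NPC blackboard on begin play.
; Its AI perception update reacts only to BP_FirstPersonCharacter actors.
; When the player is sensed it stores the actor in the blackboard's Player key, clears that key when the player is lost, and logs both changes.
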(event `self.ReceiveBeginPlay`
  (`self.UseBlackboard` "/Game/AI/BB_NPC.BB_NPC")
  (`self.RunBehaviorTree` "/Game/AI/BT_NPC.BT_NPC"))

(event `self.AIPerception.OnTargetPerceptionUpdated`
  (params (Actor :type "Actor Object Reference") (Stimulus :type "AIStimulus Structure"))
  (bind _returnvalue (`AIBlueprintHelperLibrary.GetBlackboard` null))
  (cast `/Game/FirstPerson/Blueprints/BP_FirstPersonCharacter` Actor)
  (if Stimulus_bSuccessfullySensed
    (`BlackboardComponent.SetValueAsObject` _returnvalue "Player" Actor)
    (`KismetSystemLibrary.LogString` "Player in sight")
    (else
      (`BlackboardComponent.SetValueAsObject` _returnvalue "Player" null)
      (`KismetSystemLibrary.LogString` "Player lost"))))

(fn `UserConstructionScript`)